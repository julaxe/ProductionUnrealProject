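; Enemy turret actor that tracks the player pawn, fires projectiles, and breaks once its hit count reaches its HP.
; While the player is in range, Tick smoothly rotates the Sphere toward them and accumulates a fire timer against a random delay re-rolled each frame.
; Shots spawn BulletTurretBP at the Arrow, with velocity from the Sphere's rotation offset in yaw.
; On death, the Sphere switches to physics, a sound plays, and the actor is destroyed after a delay.
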(event `self.ReceiveTick`
  (params (DeltaSeconds :type "Float (single-precision)"))
  ;[1 1 1] Event Hit - Destroy
  (if (>= (`self.TimesHitted`) (`self.HpPoints`))
    (`PrimitiveComponent.SetSimulatePhysics` (`self.Sphere`) true)
    (`PrimitiveComponent.SetCollisionEnabled` (`self.Sphere`) "PhysicsOnly")
    (`/Engine/EditorBlueprintResources/StandardMacros.DoOnce` false
      (:`Completed`
        (`GameplayStatics.PlaySoundAtLocation` "/Game/Blueprints/Sounds/Turret_Destroyed.Turret_Destroyed" (`SceneComponent.K2_GetComponentLocation` (`self.StaticMesh`)) (struct) 1.0 1.0 0.0 null null null)
        (`KismetSystemLibrary.Delay` 10.0)
        (`self.K2_DestroyActor`)))
    (elif (< (`KismetMathLibrary.Abs` (`KismetMathLibrary.Vector_Distance` (`self.K2_GetActorLocation`) (`self.K2_GetActorLocation` (`GameplayStatics.GetPlayerPawn` 0)))) 5000.0)
      (`self.AutoAim` DeltaSeconds)
      (`self.Shoot Function` DeltaSeconds (`KismetMathLibrary.RandomFloatInRange` 4.0 6.0)))))

(fn `AutoAim`
  (params (DeltaTime :type "Float (double-precision)"))
  (`SceneComponent.K2_SetWorldRotation` (`self.Sphere`) (`KismetMathLibrary.RInterpTo` (`SceneComponent.K2_GetComponentRotation` (`self.Sphere`)) (`KismetMathLibrary.FindLookAtRotation` (`SceneComponent.K2_GetComponentLocation` (`self.Sphere`)) (`self.K2_GetActorLocation` (`GameplayStatics.GetPlayerPawn` 0))) DeltaTime 2.0) false false))

(fn `Shoot Function`
  (params (deltaTime :type "Float (double-precision)") (Delay :type "Float (double-precision)"))
  (bind _output_get (set `self.TimeBullet` (+ (`self.TimeBullet`) deltaTime)))
  (if (> _output_get Delay)
    (`self.SpawnBulletTurret`)
    (`GameplayStatics.PlaySoundAtLocation` "/Game/VehicleBP/Sounds/Cannon.Cannon" (`SceneComponent.K2_GetComponentLocation` (`self.Arrow`)) (struct) 0.05 1.0 0.0 null null null)
    (set `self.TimeBullet` 0.0)))

(fn `SpawnBulletTurret`
  (bind (_returnvalue_roll _returnvalue_pitch _returnvalue_yaw) (`KismetMathLibrary.BreakRotator` (`SceneComponent.K2_GetComponentRotation` (`self.Sphere`))))
  (bind _returnvalue (`|SpawnActorFromClass` "/Game/Blueprints/BulletTurretBP.BulletTurretBP_C" (`SceneComponent.K2_GetComponentToWorld` (`self.Arrow`)) "Undefined" "OverrideRootScale" null null))
  (`ProjectileMovementComponent.SetVelocityInLocalSpace` (`/Game/Blueprints/BulletTurretBP.ProjectileMovement` _returnvalue) (* (`KismetMathLibrary.Conv_RotatorToVector` (`KismetMathLibrary.MakeRotator` _returnvalue_roll _returnvalue_pitch (+ _returnvalue_yaw -45.0))) 2000.0)))

(fn `UserConstructionScript`)