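; BulletTurretBP is a projectile actor, named as a turret bullet, that damages BP_Pickup pawns on sphere hit, then destroys itself with a fiery impact effect.
; From BeginPlay, a looping timer respawns a particle system at its location, passing BeamEnd as a vector parameter.
; A custom hit-style event, uncalled here, pushes physics bodies before delayed destruction.
; An unused Magic helper converts offset yaw into two speed-scaled components.
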(event `self.ReceiveBeginPlay`
  (`self.SpawnParticle`)
  (`KismetSystemLibrary.K2_SetTimer` null "SpawnParticle" 4.0 true))

(event `SpawnParticle`
  (bind _returnvalue (`NiagaraFunctionLibrary.SpawnSystemAtLocation` null (`self.K2_GetActorLocation`)))
  (`FXSystemComponent.SetVectorParameter` _returnvalue "New Vector" (`self.Beam End`)))

(event `CustomEvent`
  (params (MyComp :type "PrimitiveComponent Object Reference") (Other :type "Actor Object Reference") (OtherComp :type "PrimitiveComponent Object Reference") (bSelfMoved :type Boolean) (HitLocation :type "Vector Structure") (HitNormal :type "Vector Structure") (NormalImpulse :type "Vector Structure") (Hit :type "HitResult Structure (by ref)"))
  (if (`SceneComponent.IsSimulatingPhysics` OtherComp "None")
    (`PrimitiveComponent.AddForceAtLocation` OtherComp (* (`self.GetVelocity`) 1000.0) (`self.K2_GetActorLocation`) "None"))
  (`PrimitiveComponent.SetSimulatePhysics` (`self.Sphere`) true)
  (`KismetSystemLibrary.Delay` 2.0)
  (`self.K2_DestroyActor`))

(event `self.Sphere.OnComponentHit`
  (params (HitComponent :type "PrimitiveComponent Object Reference") (OtherActor :type "Actor Object Reference") (OtherComp :type "PrimitiveComponent Object Reference") (NormalImpulse :type "Vector Structure") (Hit :type "HitResult Structure (by ref)"))
  (bind _aspawn (cast `Pawn` OtherActor))
  (bind _asbp_pickup (cast `/Game/VehicleVarietyPack/Blueprints/Pickup/BP_Pickup` _aspawn))
  (`/Game/VehicleVarietyPack/Blueprints/Pickup/BP_Pickup.ReceiveDamage` _asbp_pickup)
  (`PrimitiveComponent.SetSimulatePhysics` (`self.Sphere`) true)
  (`self.K2_DestroyActor`)
  (`GameplayStatics.SpawnEmitterAtLocation` "/Game/InfinityBladeEffects/Effects/FX_Combat_Base/Impact/P_Impact_Enemy_Fire_Strong.P_Impact_Enemy_Fire_Strong" (`self.K2_GetActorLocation`) (`self.K2_GetActorRotation`) (3.0 3.0 3.0)))

(fn `Magic`
  (params (InRot :type "Rotator Structure"))
  (returns (ReturnValue :type "Float (double-precision)") (ReturnValue2 :type "Float (double-precision)"))
  (bind _speed (`self.Speed`))
  (bind _returnvalue (- (.yaw InRot) 45.0))
  (return (* (`KismetMathLibrary.DegCos` _returnvalue) _speed) (* (`KismetMathLibrary.DegSin` _returnvalue) _speed)))

(fn `UserConstructionScript`)