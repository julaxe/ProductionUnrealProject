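; Bullet projectile actor that launches along the player pawn's facing and knocks physics objects it hits.
; On BeginPlay, the Magic function turns the player's yaw, offset by 45 degrees, into a flat X/Y velocity scaled by Speed, applied in the projectile's local space.
; On hit, it applies a velocity-scaled force to simulating components, enables physics on its own cube, then destroys itself after a short delay.
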(event `self.ReceiveBeginPlay`
  (bind (_returnvalue _returnvalue2) (`self.Magic` (`self.K2_GetActorRotation` (`GameplayStatics.GetPlayerPawn` 0))))
  (`ProjectileMovementComponent.SetVelocityInLocalSpace` (`self.ProjectileMovement`) (`KismetMathLibrary.MakeVector` _returnvalue _returnvalue2)))

(event `self.ReceiveHit`
  (params (MyComp :type "PrimitiveComponent Object Reference") (Other :type "Actor Object Reference") (OtherComp :type "PrimitiveComponent Object Reference") (bSelfMoved :type Boolean) (HitLocation :type "Vector Structure") (HitNormal :type "Vector Structure") (NormalImpulse :type "Vector Structure") (Hit :type "HitResult Structure (by ref)"))
  (if (`SceneComponent.IsSimulatingPhysics` OtherComp "None")
    (`PrimitiveComponent.AddForceAtLocation` OtherComp (* (`self.GetVelocity`) 1000.0) (`self.K2_GetActorLocation`) "None"))
  (`PrimitiveComponent.SetSimulatePhysics` (`self.cubeBullet`) true)
  (`KismetSystemLibrary.Delay` 2.0)
  (`self.K2_DestroyActor`))

(fn `Magic`
  (params (InRot :type "Rotator Structure"))
  (returns (ReturnValue :type "Float (double-precision)") (ReturnValue2 :type "Float (double-precision)"))
  (bind _speed (`self.Speed`))
  (bind _returnvalue (- (.yaw InRot) 45.0))
  (return (* (`KismetMathLibrary.DegCos` _returnvalue) _speed) (* (`KismetMathLibrary.DegSin` _returnvalue) _speed)))

(fn `UserConstructionScript`)